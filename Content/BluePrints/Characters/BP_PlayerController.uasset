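; Player controller that forwards movement, look, free-look and jump input to BP_Player and manages standing, crouch and prone transitions.
; Data tables resolve each target pose and its weapon-dependent transition time, with movement locked on timed changes.
; Per-pose pitch limits gate look-up input, and a timeline rotates out-of-range views back.
; Another timeline blends spring-arm height from a table keyed by pose, with a weapon-dependent variant for moving while crouched.
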(event Custom|SetEnabled
  ;[0.15 0.15 0.15 0.5] Comment
  (Variables|Move|SetbIsEnableMove true))

(event EventBeginPlay
  (bind _asbp_player (Utilities|Casting|CastToBP_Player (Game|GetPlayerCharacter 0)))
  (Variables|Ref|SetBP_Player _asbp_player)
  (Camera|UpdatePitchLimits "NewEnumerator0")
  (EventDispatchers|BindEventtoOnMovementStateChanged (Variables|Ref|GetBP_Player) (EventDispatchers|CreateEvent :!event UpdateCameraHeight)))

(event Input|ActionEvents|InputActionFreeLook
  (params (Key :type Key%20Structure :default "None"))
  (bind _bp_player (Variables|Ref|GetBP_Player))
  ;[0.15 0.15 0.15 0.5] 모가지 꺽기
  (:Pressed
    (Default|FreeLook _bp_player true))
  (:Released
    (Default|FreeLook _bp_player false)))

(event Input|ActionEvents|InputActionCrouch
  (params (Key :type Key%20Structure :default "None"))
  (bind _bp_player (Variables|Ref|GetBP_Player))
  (bind _currentposestate (Variables|/Game/BluePrints/Characters/BP_Player.BP_Player_C|GetCurrentPoseState _bp_player))
  (bind _bisweaponequiped (Variables|/Game/BluePrints/Characters/BP_Player.BP_Player_C|GetbIsWeaponEquiped _bp_player))
  (bind (_transitiontime _topose) (CallFunction|OnTransitionTimer _bisweaponequiped "NewEnumerator1" _currentposestate))
  ;[0.15 0.15 0.15 0.5] Comment
  (:Pressed
    (CallFunction|UpdatePose _transitiontime _topose)
    (Camera|UpdatePitchLimits (Variables|/Game/BluePrints/Characters/BP_Player.BP_Player_C|GetCurrentPoseState (Variables|Ref|GetBP_Player)))
    (Camera|UpdateCameraHeight (Variables|/Game/BluePrints/Characters/BP_Player.BP_Player_C|GetbIsMovingNow (Variables|Ref|GetBP_Player)))))

(event Input|ActionEvents|InputActionProne
  (params (Key :type Key%20Structure :default "None"))
  (bind _bp_player (Variables|Ref|GetBP_Player))
  (bind _bisweaponequiped (Variables|/Game/BluePrints/Characters/BP_Player.BP_Player_C|GetbIsWeaponEquiped _bp_player))
  (bind _currentposestate (Variables|/Game/BluePrints/Characters/BP_Player.BP_Player_C|GetCurrentPoseState _bp_player))
  (bind (_transitiontime _topose) (CallFunction|OnTransitionTimer _bisweaponequiped "NewEnumerator2" _currentposestate))
  ;[0.15 0.15 0.15 0.5] Comment
  (:Pressed
    (CallFunction|UpdatePose _transitiontime _topose)
    (Camera|UpdatePitchLimits (Variables|/Game/BluePrints/Characters/BP_Player.BP_Player_C|GetCurrentPoseState (Variables|Ref|GetBP_Player)))
    (Camera|UpdateCameraHeight (Variables|/Game/BluePrints/Characters/BP_Player.BP_Player_C|GetbIsMovingNow (Variables|Ref|GetBP_Player)))))

(event Input|ActionEvents|InputActionJump
  (params (Key :type Key%20Structure :default "None"))
  (bind _bp_player (Variables|Ref|GetBP_Player))
  (bind _currentposestate (Variables|/Game/BluePrints/Characters/BP_Player.BP_Player_C|GetCurrentPoseState _bp_player))
  (bind _bisweaponequiped (Variables|/Game/BluePrints/Characters/BP_Player.BP_Player_C|GetbIsWeaponEquiped _bp_player))
  (bind (_transitiontime _topose) (CallFunction|OnTransitionTimer _bisweaponequiped "NewEnumerator0" _currentposestate))
  ;[0.15 0.15 0.15 0.5] Comment
  (:Pressed
    (if (Utilities|Enum|Equal(Enum) _currentposestate "NewEnumerator0")
      (Character|Jump (Variables|Ref|GetBP_Player))
      (else
        (CallFunction|UpdatePose _transitiontime _topose)
        (Camera|UpdateCameraHeight (Variables|/Game/BluePrints/Characters/BP_Player.BP_Player_C|GetbIsMovingNow (Variables|Ref|GetBP_Player)))))))

(event Input|AxisEvents|InputAxisTurn
  (params (AxisValue :type Float%20%28single-precision%29))
  ;[0.15 0.15 0.15 0.5] 카메라 회전
  (Default|InputTurn (Variables|Ref|GetBP_Player) AxisValue))

(event Input|AxisEvents|InputAxisLookUp
  (params (AxisValue :type Float%20%28single-precision%29))
  ;[0.15 0.15 0.15 0.5] 카메라 회전
  (bind _returnvalue (Camera|LimitPitchAngle AxisValue))
  (if _returnvalue
    (Default|InputLookUp (Variables|Ref|GetBP_Player) AxisValue)))

(event Input|AxisEvents|InputAxisMoveForward
  (params (AxisValue :type Float%20%28single-precision%29))
  ;[0.15 0.15 0.15 0.5] 캐릭터 움직이기
  (if (Variables|Move|GetbIsEnableMove)
    (Default|Move (Variables|Ref|GetBP_Player) true AxisValue)))

(event Input|AxisEvents|InputAxisMoveRight
  (params (AxisValue :type Float%20%28single-precision%29))
  ;[0.15 0.15 0.15 0.5] 캐릭터 움직이기
  (if (Variables|Move|GetbIsEnableMove)
    (Default|Move (Variables|Ref|GetBP_Player) false AxisValue)))

(event Custom|Rotate%20Speed
  (params (CurrentRotator :type Rotator) (TargetRotator :type Rotator))
  (bind _alpha (Timeline|Timeline PlayFromStart)
    (:Update
      (Pawn|SetControlRotation (Math|Rotator|Lerp(Rotator) CurrentRotator TargetRotator _alpha true)))))

(event Custom|CameraHeightSpeed
  (params (StartCamera :type Vector) (TargetCamera :type Vector))
  (bind _alpha (Timeline|Timeline_0 PlayFromStart)
    (:Update
      (Variables|/Script/Engine.SpringArmComponent|SetSocketOffset (Variables|/Game/BluePrints/Characters/BP_Player.BP_Player_C|GetSpringArm (Variables|Ref|GetBP_Player)) (Math|Vector|Lerp(Vector) StartCamera TargetCamera _alpha)))))

(fn ConstructionScript)

(fn TryGetPoseTransition
  (params (TargetPose :type E_PoseState%20Enum :default "NewEnumerator0") (FremPose :type E_PoseState%20Enum :default "NewEnumerator0"))
  (bind _returnvalue (Utilities|GetDataTableRow "/Game/BluePrints/Datas/DataTables/DT_PoseTransition.DT_PoseTransition" (Utilities|String|StringToName (Utilities|String|Append (Utilities|String|EnumtoString TargetPose) "_" (Utilities|String|EnumtoString FremPose))))
    (:then
      (return (.topose _returnvalue)))))

(fn OnTransitionTimer
  (params (bIsWeaponEqiuipped :type Boolean) (TarGetPose :type E_PoseState%20Enum :default "NewEnumerator0") (FromPose :type E_PoseState%20Enum :default "NewEnumerator0"))
  (LocalVariables|SetReturnPose (CallFunction|TryGetPoseTransition TarGetPose FromPose))
  (bind _returnvalue (Utilities|GetDataTableRow "/Game/BluePrints/Datas/DataTables/DT_ProntTime.DT_ProntTime" (Utilities|String|StringToName (Utilities|String|Append (Utilities|String|ToString(Boolean) bIsWeaponEqiuipped) "_" (Utilities|String|EnumtoString FromPose) "_" (Utilities|String|EnumtoString (LocalVariables|GetReturnPose)))))
    (:then
      _)
    (:RowNotFound
      _))
  (return (.sec _returnvalue) (LocalVariables|GetReturnPose)))

(fn UpdatePose
  (params (WaitTime :type Float%20%28double-precision%29) (To%20Pose :type E_PoseState%20Enum :default "NewEnumerator0"))
  (if (!= WaitTime 0.0)
    (Variables|Move|SetbIsEnableMove false)
    (Utilities|Time|SetTimerbyEvent (EventDispatchers|CreateEvent :!event Custom|SetEnabled) WaitTime)
    (Default|UpdatePoseState (Variables|Ref|GetBP_Player) To%20Pose)
    (else
      (Default|UpdatePoseState (Variables|Ref|GetBP_Player) To%20Pose))))

(fn UpdatePitchLimits
  (params (NewState :type E_PoseState%20Enum :default "NewEnumerator0"))
  (bind _returnvalue (Pawn|GetControlRotation :!class /Script/Engine.Controller))
  (Utilities|FlowControl|Sequence
    (:then_0
      (bind _returnvalue_2 (Utilities|GetDataTableRow "/Game/BluePrints/Datas/DataTables/DT_PichLimit.DT_PichLimit" (Utilities|String|StringToName (Utilities|String|EnumtoString NewState)))
        (:then
          (Variables|Camera|SetCachedTopLimit (.toplimit _returnvalue_2))
          (Variables|Camera|SetCachedBottomLimit (.bottomlimit _returnvalue_2)))))
    (:then_1
      ;[0.15 0.15 0.15 0.5] 현재 카메라 각도가 리밋 각도를 초과 했다면
      (if (not (or (> (.pitch _returnvalue) (Variables|Camera|GetCachedBottomLimit)) (< (.pitch _returnvalue) (Variables|Camera|GetCachedTopLimit))))
        ;[0.15 0.15 0.15 0.5] 무조건 리밋값으로 카메라를 강제 회전
        (if (< (Math|Float|Absolute(Float) (- (.pitch _returnvalue) (Variables|Camera|GetCachedTopLimit))) (Math|Float|Absolute(Float) (- (.pitch _returnvalue) (Variables|Camera|GetCachedBottomLimit))))
          (CallFunction|RotateSpeed (.CurrnetRotator (Camera|MakeViewRotator (Variables|Camera|GetCachedTopLimit))) (.TargetRotator (Camera|MakeViewRotator (Variables|Camera|GetCachedTopLimit))))
          (else
            (CallFunction|RotateSpeed (.CurrnetRotator (Camera|MakeViewRotator (Variables|Camera|GetCachedBottomLimit))) (.TargetRotator (Camera|MakeViewRotator (Variables|Camera|GetCachedBottomLimit))))))))))

(fn LimitPitchAngle
  (params (Axis :type Float%20%28double-precision%29))
  (bind _returnvalue (Class|PlayerController|GetDeprecatedInputPitchScale))
  (bind _returnvalue_2 (Pawn|GetControlRotation :!class /Script/Engine.Controller))
  (bind _returnvalue_3 (* Axis _returnvalue))
  (bind _returnvalue_4 (+ (.pitch _returnvalue_2) _returnvalue_3))
  (return (or (> _returnvalue_4 (Variables|Camera|GetCachedBottomLimit)) (< _returnvalue_4 (Variables|Camera|GetCachedTopLimit)))))

(fn MakeViewRotator
  (params (LimitPitch :type Float%20%28double-precision%29))
  (bind _returnvalue (Pawn|GetControlRotation :!class /Script/Engine.Controller))
  (bind (_roll _pitch _yaw) (Math|Rotator|BreakRotator _returnvalue))
  (return _returnvalue (Math|Rotator|MakeRotator _roll (Variables|Camera|GetCachedTopLimit) _yaw)))

(fn UpdateCameraHeight
  (params (bIsMovingNow :type Boolean))
  (bind _bp_player (Variables|Ref|GetBP_Player))
  (bind _bp_player_2 (Variables|Ref|GetBP_Player))
  (bind _currentposestate (Variables|/Game/BluePrints/Characters/BP_Player.BP_Player_C|GetCurrentPoseState _bp_player_2))
  (bind _springarm (Variables|/Game/BluePrints/Characters/BP_Player.BP_Player_C|GetSpringArm _bp_player))
  (bind _socketoffset (Variables|/Script/Engine.SpringArmComponent|GetSocketOffset _springarm))
  (Utilities|FlowControl|Sequence
    (:then_0
      (LocalVariables|SetCurrentPose (Utilities|String|EnumtoString _currentposestate))
      (if (Utilities|Enum|NotEqual(Enum) _currentposestate "NewEnumerator1")
        (LocalVariables|SetRowName (LocalVariables|GetCurrentPose))
        (else
          (LocalVariables|SetRowName (LocalVariables|GetCurrentPose))
          (if bIsMovingNow
            (LocalVariables|SetRowName (Utilities|String|Append (LocalVariables|GetRowName) "_" (Utilities|String|ToString(Boolean) (Variables|/Game/BluePrints/Characters/BP_Player.BP_Player_C|GetbIsWeaponEquiped (Variables|Ref|GetBP_Player))) "_Move"))))))
    (:then_1
      (bind _returnvalue (Utilities|GetDataTableRow "/Game/BluePrints/Datas/DataTables/DT_CamerHeight.DT_CamerHeight" (Utilities|String|StringToName (LocalVariables|GetRowName)))
        (:then
          (bind _output_get (Variables|Default|SetEndCaemra (Math|Vector|MakeVector (.x _socketoffset) (.y _socketoffset) (.height _returnvalue))))
          (CallFunction|CameraHeightSpeed (Variables|/Script/Engine.SpringArmComponent|GetSocketOffset _springarm) _output_get))))))