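; Base Blueprint for world items, holding spawn ID, serial (SN), item type, name, UI prefix and mesh.
; On BeginPlay it line-traces downward for the Land object type and snaps the actor to the hit point.
; Its Box calls begin and end overlap dispatchers only for the referenced player.
; Init functions set item data, though UIPrefix gets a fixed enum value and EnableOutline is an empty stub.
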(event OnComponentBeginOverlap(Box)
  (params (OverlappedComponent :type Primitive%20Component%20Object%20Reference) (OtherActor :type Actor%20Object%20Reference) (OtherComp :type Primitive%20Component%20Object%20Reference) (OtherBodyIndex :type Integer) (bFromSweep :type Boolean) (SweepResult :type Hit%20Result%20Structure%20%28by%20ref%29))
  (if (== OtherActor (Variables|Default|GetPlayerRef))
    (Default|CallOnBeginOverlap self)))

(event OnComponentEndOverlap(Box)
  (params (OverlappedComponent :type Primitive%20Component%20Object%20Reference) (OtherActor :type Actor%20Object%20Reference) (OtherComp :type Primitive%20Component%20Object%20Reference) (OtherBodyIndex :type Integer))
  (if (== OtherActor (Variables|Default|GetPlayerRef))
    (Default|CallOnEndOverlap self)))

(event EventBeginPlay
  (bind _returnvalue (Transformation|GetActorLocation))
  ;[0.15 0.15 0.15 0.5] 아랫 방향으로 라인트레이스를 쏴서 "오브 젝트 타입"이 Land 인 녀석만 감지해서 해당 레이저가 맞은 위치로 지금 이 엑터의 좌표를 변경해주세요
  (|CallParentFunction)
  (bind (_outhit _returnvalue_2) (Collision|LineTraceForObjects _returnvalue (+ _returnvalue (* (Math|Vector|VectorDown) 1e+03)) (Utilities|Array|MakeArray "ObjectTypeQuery7") false 0 "ForDuration"))
  (if _returnvalue_2
    (Transformation|SetActorLocation (.Location (Collision|BreakHitResult _outhit)) false false)))

(fn ConstructionScript
  (|CallParentFunction))

(fn InitSpawnData
  (params (ID :type Name) (SN :type String))
  (Variables|Default|SetID ID)
  (Variables|Default|SetSN SN))

(fn InitWorldItemBaseData
  (params (ItemType :type E_ItemType%20Enum :default "NewEnumerator0") (ItemName :type Text) (UIPrefix :type E_ItemType%20Enum :default "NewEnumerator0") (StaticMesh :type E_ItemType%20Enum :default "NewEnumerator0"))
  (Variables|Default|SetItemType ItemType)
  (Variables|Default|SetItemName ItemName)
  (Variables|Default|SetUIPrefix (Utilities|Enum|ByteToEnumNewUserDefinedEnum))
  (Components|StaticMesh|SetStaticMesh (Variables|Default|GetStaticMesh) 0))

(fn EnableOutline)