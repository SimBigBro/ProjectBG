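; BP_WorldItem_Boost is the world item actor for boost items, specializing a parent world item class.
; InitSpwanData calls the parent, then looks up the given ID in DT_WorldItem_BoostData to initialize base type, name, UI prefix and static mesh, and to store the per-unit weight.
; GetWeight returns Amount times that unit weight.
; The event graph has no active logic.
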(event EventBeginPlay
  (|CallParentFunction) ; This node is disabled and will not be called.\nDrag off pins to build functionality.
)

(event Collision|EventActorBeginOverlap
  (params (OtherActor :type Actor%20Object%20Reference)))

(event EventTick
  (params (DeltaSeconds :type Float%20%28single-precision%29)))

(fn ConstructionScript
  (|CallParentFunction))

(fn InitSpwanData
  (params (ID :type Name :default "None") (SN :type String))
  (|CallParentFunction ID SN)
  (bind _returnvalue (Utilities|GetDataTableRow "/Game/Blueprints/Datas/DataTable/Item/DT_WorldItem_BoostData.DT_WorldItem_BoostData" (Variables|Default|GetID))
    (:then
      (CallFunction|InitWroldItemBaseData (.itemtype _returnvalue) (.itemname _returnvalue) (.uiprefix _returnvalue) (.staticmesh _returnvalue))
      (Variables|Default|SetSingleWeight (.weight _returnvalue)))))

(fn GetWeight
  (return (* (Variables|Default|GetAmount) (Variables|Default|GetSingleWeight))))