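; Game mode that scatters randomized loot across the map on BeginPlay, spawning an item group at each DT_ItemGroupLocation row.
; Each group rolls an item count, re-rolls until that many distinct types are chosen, then picks an ID per type from its probability table.
; Count and ID use cumulative percentages, while type draws from a percent-weighted array.
; The matching world item class spawns at each random group transform and receives its ID.
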(event EventBeginPlay
  (CallFunction|GenerateItems))

(fn ConstructionScript)

(fn GenerateItems
  (bind _outrownames (DataTable|GetDataTableRowNames "/Game/Blueprints/Datas/DataTable/ItemGeneration/DT_ItemGroupLocation.DT_ItemGroupLocation"))
  (for _array_element _outrownames
    (bind _returnvalue (Utilities|GetDataTableRow "/Game/Blueprints/Datas/DataTable/ItemGeneration/DT_ItemGroupLocation.DT_ItemGroupLocation" _array_element)
      (:then
        (bind _returnvalue_2 (Game|SpawnActorfromClass "/Game/Blueprints/Items/BP_ItemGruop.BP_ItemGruop_C" (Math|Transform|MakeTransform (.location _returnvalue) "0, 0, 0" "1.000000,1.000000,1.000000") "Undefined" "MultiplyWithRoot" 0 0))
        (Variables|Default|SetItemGroupRef _returnvalue_2)
        (Utilities|Array|Clear (LocalVariables|GetItemTypeArr))
        (bind _number (CallFunction|RandomItemNumber))
        (LocalVariables|SetSpawnTransforms (Default|GetRandomTransforms (Variables|Default|GetItemGroupRef) _number))
        (for _index (range 1 _number)
          (bind _itemtype (CallFunction|RandomItemType :!label _label))
          (if (== (Utilities|Array|FindItem (LocalVariables|GetItemTypeArr) _itemtype) -1)
            (Utilities|Array|Add (LocalVariables|GetItemTypeArr) _itemtype)
            (else
              (goto _label))))
        (for _array_element_2 (LocalVariables|GetItemTypeArr)
          (bind _st_spawnitem (CallFunction|RandomItemId _array_element_2))
          (Utilities|Array|Add (LocalVariables|GetSpawnItemArr) _st_spawnitem))
        (for (_array_element_3 _array_index) (LocalVariables|GetSpawnItemArr)
          (bind _output_get (LocalVariables|SetSpawnItemType (.itemtype _array_element_3)))
          (LocalVariables|SetSpawnItemID (.id _array_element_3))
          (bind _returnvalue_3 (Game|SpawnActorfromClass (Utilities|Select :Index _output_get :NewEnumerator0 "/Game/Blueprints/Items/WolrdItems/BP_WorldItem_Weapon.BP_WorldItem_Weapon_C" :NewEnumerator1 "/Game/Blueprints/Items/WolrdItems/BP_WorldItem_Acc.BP_WorldItem_Acc_C" :NewEnumerator2 "/Game/Blueprints/Items/WolrdItems/BP_WorldItem_Ammo.BP_WorldItem_Ammo_C" :NewEnumerator3 "/Game/Blueprints/Items/WolrdItems/BP_WorldItem_Health.BP_WorldItem_Health_C" :NewEnumerator4 "/Game/Blueprints/Items/WolrdItems/BP_WorldItem_Boost.BP_WorldItem_Boost_C" :NewEnumerator5 "/Game/Blueprints/Items/WolrdItems/BP_WroldItem_Helmet.BP_WroldItem_Helmet_C" :NewEnumerator6 "/Game/Blueprints/Items/WolrdItems/BP_WroldItem_Vest.BP_WroldItem_Vest_C" :NewEnumerator7 "/Game/Blueprints/Items/WolrdItems/BP_WroldItem_Backpack.BP_WroldItem_Backpack_C") (Utilities|Array|Get(acopy) (LocalVariables|GetSpawnTransforms) _array_index) "Undefined" "MultiplyWithRoot" 0 0))
          (bind _asbp_world_item_base (Utilities|Casting|CastToBP_WorldItemBase _returnvalue_3))
          (Default|InitSpwanData _asbp_world_item_base (LocalVariables|GetSpawnItemID) "1"))
        (Utilities|Array|Clear (LocalVariables|GetSpawnItemArr))
        (Utilities|Array|Clear (LocalVariables|GetSpawnTransforms))))))

(fn RandomItemNumber
  ;[0.15 0.15 0.15 0.5] 최악의 가정하에 6번
  (bind _outrownames (DataTable|GetDataTableRowNames "/Game/Blueprints/Datas/DataTable/ItemGeneration/DT_NumberProbability.DT_NumberProbability"))
  (for _array_element _outrownames
    ;;[0.15 0.15 0.15 0.5] 3번
    (bind _returnvalue (Utilities|GetDataTableRow "/Game/Blueprints/Datas/DataTable/ItemGeneration/DT_NumberProbability.DT_NumberProbability" _array_element)
      (:then
        (LocalVariables|SetTotalPercent (+ (LocalVariables|GetTotalPercent) (.percent _returnvalue))))))
  (LocalVariables|SetRandomValue (Math|Random|RandomIntegerinRange 1 (LocalVariables|GetTotalPercent)))
  ;;[0.15 0.15 0.15 0.5] 1~3번
  (for _array_element_2 _outrownames
    (bind _returnvalue_2 (Utilities|GetDataTableRow "/Game/Blueprints/Datas/DataTable/ItemGeneration/DT_NumberProbability.DT_NumberProbability" _array_element_2)
      (:then
        (bind _output_get (LocalVariables|SetSumPercent (+ (LocalVariables|GetSumPercent) (.percent _returnvalue_2))))
        (if (>= _output_get (LocalVariables|GetRandomValue))
          (return (.number _returnvalue_2)))))))

(fn RandomItemType
  (bind _outrownames (DataTable|GetDataTableRowNames "/Game/Blueprints/Datas/DataTable/ItemGeneration/DT_ItemTypeProbability.DT_ItemTypeProbability"))
  (for _array_element _outrownames
    (bind _returnvalue (Utilities|GetDataTableRow "/Game/Blueprints/Datas/DataTable/ItemGeneration/DT_ItemTypeProbability.DT_ItemTypeProbability" _array_element)
      (:then
        (for _index (range 1 (.percent _returnvalue))
          (Utilities|Array|Add (LocalVariables|GetItemTypeArr) (.itemtype _returnvalue))))))
  (return (.OutItem (Utilities|Array|Random (LocalVariables|GetItemTypeArr)))))

(fn RandomItemId
  (params (ItemType :type E_ItemType%20Enum :default "NewEnumerator0"))
  (bind _returnvalue (Utilities|Select :Index ItemType :NewEnumerator0 "/Game/Blueprints/Datas/DataTable/ItemGeneration/DT_WeaponProbability.DT_WeaponProbability" :NewEnumerator1 "/Game/Blueprints/Datas/DataTable/ItemGeneration/DT_AccProbability.DT_AccProbability" :NewEnumerator2 "/Game/Blueprints/Datas/DataTable/ItemGeneration/DT_AmmoProbability.DT_AmmoProbability" :NewEnumerator3 "/Game/Blueprints/Datas/DataTable/ItemGeneration/DT_HealthProbability.DT_HealthProbability" :NewEnumerator4 "/Game/Blueprints/Datas/DataTable/ItemGeneration/DT_BoostProbability.DT_BoostProbability" :NewEnumerator5 "/Game/Blueprints/Datas/DataTable/ItemGeneration/DT_HelmetProbability.DT_HelmetProbability" :NewEnumerator6 "/Game/Blueprints/Datas/DataTable/ItemGeneration/DT_VestProbability.DT_VestProbability" :NewEnumerator7 "/Game/Blueprints/Datas/DataTable/ItemGeneration/DT_BackpackProbability.DT_BackpackProbability"))
  ;[0.15 0.15 0.15 0.5] 들어온 아이템 타입에 따라 데이터 테이블 선택
  (Utilities|FlowControl|Sequence
    (:then_0
      (bind _outrownames (DataTable|GetDataTableRowNames _returnvalue))
      (for _array_element _outrownames
        ;[0.15 0.15 0.15 0.5] 데이터테이블에 따라 정해진 확률대로 배열에 채우기
        (bind _returnvalue_2 (Utilities|GetDataTableRow _returnvalue _array_element)
          (:then
            (bind _output_get (LocalVariables|SetSumPercent (+ (LocalVariables|GetSumPercent) (Utilities|Struct|BreakST_ItemProbability _returnvalue_2))))
            (if (>= _output_get (LocalVariables|GetRandomValue))
              (return (Utilities|Struct|MakeST_SpawnItem ItemType _array_element)))))))))